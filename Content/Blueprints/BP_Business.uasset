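; Controller actor for the WanLi scene that switches between the streamed city and interior levels and plays their level sequences.
; Level switches show a LOGO widget and reset the PSFreeCameraPawn view.
; PlaySeqence waits a fixed 3 seconds after loading, hides the logo, then plays a sequence found by tag or class.
; Anim Combine chains Outside_Out, interior and Outside_In via OnFinished, and CurrentSeq supports pause and stop.
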(event Custom|LoadLevel
  (params (Name :type Name))
  (Game|UnloadStreamLevel(byName) (Variables|Default|GetCurrentLevelName) false)
  (Game|LoadStreamLevel(byName) Name true)
  (Variables|Default|SetCurrentLevelName Name))

(event Custom|PlaySeqence
  (params (sequence :type String))
  (switch string sequence
    (:Inside
      (CallFunction|PlayInside))
    (:Outside_In
      (CallFunction|PlayOutsidein))
    (:Outside_Out
      (CallFunction|PlayOutsideOut))
    (:AnimCombine
      (CallFunction|LoadOutsideLevel)
      (Utilities|FlowControl|Delay 3.0)
      (CallFunction|ShowLogo false)
      (bind _outactors (Actor|GetAllActorswithTag "Outside_Out"))
      (bind _aslevel_sequence_actor (Utilities|Casting|CastToLevelSequenceActor (Utilities|Array|Get(acopy) _outactors)))
      (bind _output_get (Variables|Default|SetCurrentSeq _aslevel_sequence_actor))
      (Sequencer|Player|Play (Variables|/Script/LevelSequence.LevelSequenceActor|GetSequencePlayer _output_get) :!class /Script/MovieScene.MovieSceneSequencePlayer)
      (EventDispatchers|AssignOnFinished (Variables|/Script/LevelSequence.LevelSequenceActor|GetSequencePlayer _output_get) (delegate Custom|OnFinished_Event)))))

(event Custom|PlayOutside_in
  (CallFunction|LoadOutsideLevel)
  (Utilities|FlowControl|Delay 3.0)
  (CallFunction|ShowLogo false)
  (bind _outactors (Actor|GetAllActorswithTag "Outside_In"))
  (bind _aslevel_sequence_actor (Utilities|Casting|CastToLevelSequenceActor (Utilities|Array|Get(acopy) _outactors)))
  (bind _output_get (Variables|Default|SetCurrentSeq _aslevel_sequence_actor))
  (Sequencer|Player|Play (Variables|/Script/LevelSequence.LevelSequenceActor|GetSequencePlayer _output_get) :!class /Script/MovieScene.MovieSceneSequencePlayer))

(event Custom|PlayInside
  (CallFunction|LoadInsideLevel)
  (Utilities|FlowControl|Delay 3.0)
  (CallFunction|ShowLogo false)
  (bind _returnvalue (Actor|GetActorOfClass "/Script/LevelSequence.LevelSequenceActor"))
  (Variables|Default|SetCurrentSeq _returnvalue)
  (Sequencer|Player|Play (Variables|/Script/LevelSequence.LevelSequenceActor|GetSequencePlayer _returnvalue) :!class /Script/MovieScene.MovieSceneSequencePlayer))

(event Custom|PlayOutside_out
  (CallFunction|LoadOutsideLevel)
  (Utilities|FlowControl|Delay 3.0)
  (CallFunction|ShowLogo false)
  (bind _outactors (Actor|GetAllActorswithTag "Outside_Out"))
  (bind _aslevel_sequence_actor (Utilities|Casting|CastToLevelSequenceActor (Utilities|Array|Get(acopy) _outactors)))
  (bind _output_get (Variables|Default|SetCurrentSeq _aslevel_sequence_actor))
  (Sequencer|Player|Play (Variables|/Script/LevelSequence.LevelSequenceActor|GetSequencePlayer _output_get) :!class /Script/MovieScene.MovieSceneSequencePlayer))

(event Custom|OnFinished_Event
  (CallFunction|LoadInsideLevel)
  (Utilities|FlowControl|Delay 3.0)
  (CallFunction|ShowLogo false)
  (bind _returnvalue (Actor|GetActorOfClass "/Script/LevelSequence.LevelSequenceActor"))
  (Variables|Default|SetCurrentSeq _returnvalue)
  (Sequencer|Player|Play (Variables|/Script/LevelSequence.LevelSequenceActor|GetSequencePlayer _returnvalue) :!class /Script/MovieScene.MovieSceneSequencePlayer)
  (EventDispatchers|AssignOnFinished (Variables|/Script/LevelSequence.LevelSequenceActor|GetSequencePlayer _returnvalue) (delegate Custom|OnFinished_Event_0)))

(event Custom|OnFinished_Event_0
  (CallFunction|LoadOutsideLevel)
  (Utilities|FlowControl|Delay 3.0)
  (CallFunction|ShowLogo false)
  (bind _outactors (Actor|GetAllActorswithTag "Outside_In"))
  (bind _aslevel_sequence_actor (Utilities|Casting|CastToLevelSequenceActor (Utilities|Array|Get(acopy) _outactors)))
  (bind _output_get (Variables|Default|SetCurrentSeq _aslevel_sequence_actor))
  (Sequencer|Player|Play (Variables|/Script/LevelSequence.LevelSequenceActor|GetSequencePlayer _output_get) :!class /Script/MovieScene.MovieSceneSequencePlayer))

(event Custom|LoadOutsideLevel
  (if (!= (Variables|Default|GetCurrentLevelName) "WanLi_City")
    (CallFunction|ShowLogo true)
    (Game|UnloadStreamLevel(byName) (Variables|Default|GetCurrentLevelName) false)
    (Game|LoadStreamLevel(byName) "WanLi_City" true)
    (Variables|Default|SetCurrentLevelName "WanLi_City")
    (CallFunction|SetViewPort "0, 0, 0" "-40.000000,60.000000,0.000000" 8e+04)))

(event Custom|LoadInsideLevel
  (if (!= (Variables|Default|GetCurrentLevelName) "WanLi_Inside")
    (CallFunction|ShowLogo true)
    (Game|UnloadStreamLevel(byName) (Variables|Default|GetCurrentLevelName) false)
    (Game|LoadStreamLevel(byName) "WanLi_Inside" true)
    (Variables|Default|SetCurrentLevelName "WanLi_Inside")
    (CallFunction|SetViewPort "0, 0, 0" "-40.000000,60.000000,0.000000" 8e+04)))

(event Custom|SetViewPort
  (params (LookPoint :type Vector) (ViewAngle :type Rotator) (Dis :type Float%20%28double-precision%29))
  (Class|FreeCameraPawn|SetLookPointAngleDistance (Variables|Default|GetPawn) LookPoint ViewAngle Dis true))

(event Custom|StopAnim
  (bind _currentseq (Variables|Default|GetCurrentSeq))
  (Utilities|IsValid _currentseq
    (:Is%20Valid
      (Sequencer|Player|Stop (Variables|/Script/LevelSequence.LevelSequenceActor|GetSequencePlayer _currentseq) :!class /Script/MovieScene.MovieSceneSequencePlayer))))

(event Custom|PauseAnim
  (bind _currentseq (Variables|Default|GetCurrentSeq))
  (Utilities|IsValid _currentseq
    (:Is%20Valid
      (Sequencer|Player|Pause (Variables|/Script/LevelSequence.LevelSequenceActor|GetSequencePlayer _currentseq)))))

(event Custom|ShowLogo
  (params (show :type Boolean))
  (bind _logo (Variables|Default|GetLOGO))
  (if show
    (Widget|SetVisibility _logo "Visible")
    (else
      (Widget|SetVisibility _logo "Hidden"))))

(event EventBeginPlay
  (CallFunction|LoadOutsideLevel)
  (bind _returnvalue (Actor|GetActorOfClass "/Game/Blueprints/Pawn/PSFreeCameraPawn.PSFreeCameraPawn_C"))
  (Variables|Default|SetPawn _returnvalue)
  (bind _returnvalue_2 (UserInterface|CreateWidget "/Game/Blueprints/LOGO.LOGO_C"))
  (bind _output_get (Variables|Default|SetLOGO _returnvalue_2))
  (UserInterface|Viewport|AddtoViewport _output_get 0)
  (Widget|SetVisibility _output_get "Hidden"))

(event Collision|EventActorBeginOverlap
  (params (OtherActor :type Actor%20Object%20Reference)))

(event EventTick
  (params (DeltaSeconds :type Float%20%28single-precision%29)))

(fn ConstructionScript)