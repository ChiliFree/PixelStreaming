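; Player controller for a Pixel Streaming demo that handles browser commands and cycles feature showcase levels.
; At BeginPlay it finds BP_CharConfig and binds Pixel Streaming input, routing JSON fields to character or skin changes on that actor, or to an r.setres resolution change.
; Pressing F fades the camera out, updates the HUD's feature UI, hides all feature sublevels, shows the selected one and fades back in, guarded by IsTransitioning.
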(event Custom|OnJSONEvent
  (params (Descriptor :type String))
  ;[1 1 1] Bind JSON events - This is listening for HTML/JavaScript events from the Pixel Streaming client's web browser.
  (Variables|Default|SetDescriptor Descriptor)
  (if (.Success (Class|PixelStreamingInput|GetJsonStringValue (Variables|Default|GetPixelStreamingInput) (Variables|Default|GetDescriptor) "Character"))
    (CallFunction|ChangeCharacter)
    (elif (.Success (Class|PixelStreamingInput|GetJsonStringValue (Variables|Default|GetPixelStreamingInput) (Variables|Default|GetDescriptor) "Skin"))
      (CallFunction|ChangeSkin)
      (elif (.Success (Class|PixelStreamingInput|GetJsonStringValue (Variables|Default|GetPixelStreamingInput) (Variables|Default|GetDescriptor) "Resolution"))
        (CallFunction|ChangeResolution)))))

(event Custom|TurnOffLevels
  ;[1 1 1] Turn off all sub levels while switching levels
  (for _array_element (Variables|Default|GetFeatureMaps)
    (Utilities|IsValid (Class|GameplayStatics|GetStreamingLevel (Utilities|String|StringToName _array_element))
      (:Is%20Valid
        (Variables|/Script/Engine.LevelStreaming|SetbShouldBeVisible (Class|GameplayStatics|GetStreamingLevel (Utilities|String|StringToName _array_element)) false)))))

(event Custom|ChangeResolution
  (bind _descriptor (Variables|Default|GetDescriptor))
  (bind _pixelstreaminginput (Variables|Default|GetPixelStreamingInput))
  (bind _descriptor_2 (Variables|Default|GetDescriptor))
  (bind _pixelstreaminginput_2 (Variables|Default|GetPixelStreamingInput))
  (bind (_stringvalue _success) (Class|PixelStreamingInput|GetJsonStringValue _pixelstreaminginput _descriptor "X"))
  (bind (_stringvalue_2 _success_2) (Class|PixelStreamingInput|GetJsonStringValue _pixelstreaminginput_2 _descriptor_2 "Y"))
  ;[1 1 1] JSON Event: Resolution
  (if _success
    (if _success_2
      (Development|ExecuteConsoleCommand (Utilities|String|Append "r.setres " _stringvalue "x" _stringvalue_2) 0))))

(event Custom|ChangeCharacter
  (bind _descriptor (Variables|Default|GetDescriptor))
  (bind _pixelstreaminginput (Variables|Default|GetPixelStreamingInput))
  (bind _stringvalue (Class|PixelStreamingInput|GetJsonStringValue _pixelstreaminginput _descriptor "Character"))
  ;[1 1 1] Change Character
  (if true
    (Development|PrintString _stringvalue false true "(R=1.000000,G=0.409627,B=0.000000,A=1.000000)" 2e+01)
    (Default|ChangeCharacter (Variables|Default|GetCharConfigRef) _stringvalue)))

(event Custom|ChangeSkin
  (bind _descriptor (Variables|Default|GetDescriptor))
  (bind _pixelstreaminginput (Variables|Default|GetPixelStreamingInput))
  (bind (_stringvalue _success) (Class|PixelStreamingInput|GetJsonStringValue _pixelstreaminginput _descriptor "Skin"))
  ;[1 1 1] Change Skin
  (if _success
    (Default|ChangeSkin (Variables|Default|GetCharConfigRef) (Math|Conversions|ToInteger(Byte) _stringvalue))))

(event EventBeginPlay
  ;[1 1 1] Begin Play
  (bind _asbp_orbit_pawn (Utilities|Casting|CastToBP_Orbit_Pawn (Game|Player|GetPlayerPawn 0)))
  (Variables|Default|SetPlayerPawn _asbp_orbit_pawn)
  (bind _outactors (Actor|GetAllActorsOfClass "/Game/Blueprints/CharacterConfig/BP_CharConfig.BP_CharConfig_C"))
  (for _array_element _outactors
    (Variables|Default|SetCharConfigRef _array_element))
  ;[1 1 1] Bind JSON events - This is listening for HTML/JavaScript events from the Pixel Streaming client's web browser.
  (EventDispatchers|BindEventtoOnInputEvent (Variables|Default|GetPixelStreamingInput) (delegate Custom|OnJSONEvent)))

(event Input|KeyboardEvents|F
  (params (Key :type Key%20Structure))
  ;[1 1 1] Change Pixel Streaming feature by pressing 'F'
  (:Pressed
    (if (not (Variables|Default|GetIsTransitioning))
      (Variables|Default|SetMapSelection (Utilities|Array|Get(acopy) (Variables|Default|GetFeatureMaps) (Variables|Default|GetSelectedMapIdx)))
      (Variables|Default|SetSelectedMapIdx (Math|Integer|%(Integer) (+ (Variables|Default|GetSelectedMapIdx) 1) (Utilities|Array|Length (Variables|Default|GetFeatureMaps))))
      (Variables|Default|SetIsTransitioning true)
      (CameraFades|StartCameraFade :self (Game|GetPlayerCameraManager 0) :ToAlpha 1.0 :Duration 0.5 :bShouldFadeAudio true :bHoldWhenFinished true)
      (bind _asnew_hud (Utilities|Casting|CastToNewHUD (HUD|GetHUD (Game|GetPlayerController 0))))
      (Default|UpdateFeatureUI (Variables|/Game/Blueprints/PixelStreaming/NewHUD.NewHUD_C|GetUI%20Ref _asnew_hud) (Variables|Default|GetMapSelection))
      (Utilities|FlowControl|Delay 0.7)
      (CallFunction|TurnOffLevels)
      (Utilities|IsValid (Class|GameplayStatics|GetStreamingLevel (Utilities|String|StringToName (Variables|Default|GetMapSelection)))
        (:Is%20Valid
          (Variables|/Script/Engine.LevelStreaming|SetbShouldBeVisible (Class|GameplayStatics|GetStreamingLevel (Utilities|String|StringToName (Variables|Default|GetMapSelection))) true)
          (CameraFades|StartCameraFade :self (Game|GetPlayerCameraManager 0) :FromAlpha 1.0 :Duration 0.5 :bShouldFadeAudio true)
          (Utilities|FlowControl|Delay 0.5)
          (Variables|Default|SetIsTransitioning false))))))

(fn ConstructionScript)