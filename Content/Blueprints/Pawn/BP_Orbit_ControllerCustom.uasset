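; Orbit controller that receives JSON input events from a Pixel Streaming browser client.
; On BeginPlay it caches the orbit pawn, binds the input listener, then routes events by Character, Skin or Resolution field.
; Only Resolution acts, running r.setres with the sent X and Y.
; Character and skin handlers are empty; their BP_CharConfig logic and a faded feature-map switcher remain as disconnected nodes.
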(event Custom|OnJSONEvent
  (params (Descriptor :type String))
  ;[1 1 1] Bind JSON events - This is listening for HTML/JavaScript events from the Pixel Streaming client's web browser.
  (bind _output_get (Variables|Default|SetDescriptor Descriptor))
  (Development|PrintString _output_get)
  (if (.Success (Class|PixelStreamingInput|GetJsonStringValue (Variables|Default|GetPixelStreamingInput) (Variables|Default|GetDescriptor) "Character"))
    (CallFunction|ChangeCharacter)
    (elif (.Success (Class|PixelStreamingInput|GetJsonStringValue (Variables|Default|GetPixelStreamingInput) (Variables|Default|GetDescriptor) "Skin"))
      (CallFunction|ChangeSkin)
      (elif (.Success (Class|PixelStreamingInput|GetJsonStringValue (Variables|Default|GetPixelStreamingInput) (Variables|Default|GetDescriptor) "Resolution"))
        (CallFunction|ChangeResolution)))))

(event Custom|TurnOffLevels
  ;[1 1 1] Turn off all sub levels while switching levels
  (for _array_element (Variables|Default|GetFeatureMaps)
    (Utilities|IsValid (Class|GameplayStatics|GetStreamingLevel (Utilities|String|StringToName _array_element))
      (:Is%20Valid
        (Variables|/Script/Engine.LevelStreaming|SetbShouldBeVisible (Class|GameplayStatics|GetStreamingLevel (Utilities|String|StringToName _array_element)) false)))))

(event Custom|ChangeResolution
  (bind _descriptor (Variables|Default|GetDescriptor))
  (bind _pixelstreaminginput (Variables|Default|GetPixelStreamingInput))
  (bind _descriptor_2 (Variables|Default|GetDescriptor))
  (bind _pixelstreaminginput_2 (Variables|Default|GetPixelStreamingInput))
  (bind (_stringvalue _success) (Class|PixelStreamingInput|GetJsonStringValue _pixelstreaminginput _descriptor "X"))
  (bind (_stringvalue_2 _success_2) (Class|PixelStreamingInput|GetJsonStringValue _pixelstreaminginput_2 _descriptor_2 "Y"))
  ;[1 1 1] JSON Event: Resolution
  (if _success
    (if _success_2
      (Development|ExecuteConsoleCommand (Utilities|String|Append "r.setres " _stringvalue "x" _stringvalue_2) 0))))

(event Custom|ChangeCharacter
  ;[1 1 1] Change Character
)

(event Custom|ChangeSkin
  ;[1 1 1] Change Skin
)

(event EventBeginPlay
  ;[1 1 1] Begin Play
  (bind _asbp_orbit_pawn (Utilities|Casting|CastToBP_Orbit_Pawn (Game|Player|GetPlayerPawn 0)))
  (Variables|Default|SetPlayerPawn _asbp_orbit_pawn)
  ;[1 1 1] Bind JSON events - This is listening for HTML/JavaScript events from the Pixel Streaming client's web browser.
  (EventDispatchers|BindEventtoOnInputEvent (Variables|Default|GetPixelStreamingInput) (delegate Custom|OnJSONEvent)))

(event Input|KeyboardEvents|F
  (params (Key :type Key%20Structure :default "None"))
  ;[1 1 1] Change Pixel Streaming feature by pressing 'F'
)

(fn ConstructionScript)